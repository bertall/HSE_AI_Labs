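; Bonus pickup that adds score to the game state when it hits the paddle.
; SetBonus picks a red or blue sprite with a matching score value.
; On collection, a guard blocks repeats, the sprite gives way to "+score" text, and the collision body's velocity is reset.
; A mass-scaled impulse pops it upward and randomly sideways before the actor destroys itself after a short delay.
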(event `CollectBonus`
  (bind _collision (`self.Collision`))
  (bind _returnvalue (* (`KismetMathLibrary.SignOfFloat` (`KismetMathLibrary.RandomFloatInRange` -1.0 1.0)) (* (`PrimitiveComponent.GetMass` _collision) 50.0)))
  ;[1 1 1] Collect Bonus Custom event
  (if (not (`self.isCollected`))
    (set `self.isCollected` true)
    (message `/Game/BluePrints/InterfacesBP/Score_Lives_BP_Interface.UpdateScore` (`GameplayStatics.GetGameState`) (`self.ScoreToAdd`))
    (`SceneComponent.SetVisibility` (`self.BonusSprite`) false false)
    (`SceneComponent.SetVisibility` (`self.BonusText`) true false)
    (`PrimitiveComponent.SetAllPhysicsLinearVelocity` _collision (0.0 0.0 0.0) false)
    (`PrimitiveComponent.AddImpulse` _collision (`KismetMathLibrary.MakeVector` _returnvalue 0.0 (/ (`KismetMathLibrary.Abs` _returnvalue) 2.0)) "None" true)
    (`TextRenderComponent.K2_SetText` (`self.BonusText`) (`KismetTextLibrary.Conv_StringToText` (`KismetStringLibrary.Concat_StrStr` "+" (`KismetStringLibrary.Conv_IntToString` (`self.ScoreToAdd`)))))
    (`KismetSystemLibrary.Delay` 0.5)
    (`self.K2_DestroyActor`)))

(event `SetBonus`
  (params (Type :type "/Game/BluePrints/Enums/BonusType Enum" :default "NewEnumerator0"))
  ;[1 1 1] Set Bunus Custom Event
  (switch `/Game/BluePrints/Enums/BonusType` Type
    (:`NewEnumerator1`
      (set `self.Sprite` "/Game/Assets/NewFolder/element_red_polygon_Sprite.element_red_polygon_Sprite")
      (set `self.ScoreToAdd` 50))
    (:`NewEnumerator2`
      (set `self.Sprite` "/Game/Assets/NewFolder/element_blue_polygon_Sprite.element_blue_polygon_Sprite")
      (set `self.ScoreToAdd` 20)))
  (`PaperSpriteComponent.SetSprite` (`self.BonusSprite`) (`self.Sprite`)))

(event `self.ReceiveHit`
  (params (MyComp :type "PrimitiveComponent Object Reference") (Other :type "Actor Object Reference") (OtherComp :type "PrimitiveComponent Object Reference") (bSelfMoved :type Boolean) (HitLocation :type "Vector Structure") (HitNormal :type "Vector Structure") (NormalImpulse :type "Vector Structure") (Hit :type "HitResult Structure (by ref)"))
  ;[1 1 1] Overlap Event
  (cast `/Game/BluePrints/Paddle_BP` Other)
  (`self.CollectBonus`))

(fn `RemoveLives`
  (params (Value :type Integer))
  (return))

(fn `UserConstructionScript`)