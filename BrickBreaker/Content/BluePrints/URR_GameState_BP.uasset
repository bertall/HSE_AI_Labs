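; Game state Blueprint that tracks score and lives and reloads Level1Map when a lives check fails.
; Interface events add to the score and write it to the HUD text, or add and remove lives with clamping at zero.
; Both lives events share the check, apparently a math expression testing RealLives.
; The HUD lives-texture update is disconnected, so only score reaches the display.
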(event EventUpdateScore
  (params (Value :type Integer))
  ;[1 1 1] Update Score event (Interface)
  (bind _output_get (Variables|Default|SetScore (+ Value (Variables|Default|GetScore))))
  (Rendering|Components|TextRender|SetText (Variables|/Game/BluePrints/WidgetsBP/InGameHUD_WG.InGameHUD_WG_C|GetScoreText (Variables|Default|GetInGameHUD_WG_Ref)) (Utilities|Text|ToText(String) (Utilities|String|Append "" (Utilities|String|ToString(Integer) _output_get)))))

(event EventAddLives
  (params (value :type Integer))
  ;[1 1 1] Add Lives Event(Interface)
  (Variables|Default|SetRealLives (Math|Integer|Clamp(Integer) (+ value (Variables|Default|GetRealLives)) 0 1000000))
  (if (not (|({7E960BBA-473F-EC65-07E8-1382F7E69ACA}>1)))
    (Game|OpenLevel(byName) "Level1Map")))

(event EventRemoveLives
  (params (Value :type Integer))
  ;[1 1 1] Remove Lives Event (Interface)
  (Variables|Default|SetRealLives (Math|Integer|Clamp(Integer) (- (Variables|Default|GetRealLives) Value) 0 1000000))
  (if (not (|({7E960BBA-473F-EC65-07E8-1382F7E69ACA}>1)))
    (Game|OpenLevel(byName) "Level1Map")))

(fn ConstructionScript)