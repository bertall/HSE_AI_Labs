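; Paddle actor that slides along its forward axis, driven by an integer Action set outside this graph.
; BeginPlay sets the speed, clears GameStarted, spawns and stores a ScreenCapturer_BP, and caches the URR game state.
; Tick maps Action to MoveLeft or MoveRight, which apply swept, delta-time-scaled movement only while GameStarted is true.
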(event `self.ReceiveBeginPlay`
  ;[1 1 1] Begin Play Event(Initialization)
  (set `self.Speed` 750.0)
  (set `self.GameStarted` false)
  (`|ExecutionSequence`
    (:`then_0`
      (bind _returnvalue (`|SpawnActorFromClass` "/Game/BluePrints/ScreenCapturer_BP.ScreenCapturer_BP_C" (`KismetMathLibrary.MakeTransform` (0.0 0.0 0.0)) "Undefined" "OverrideRootScale"))
      (set `self.ScreenCapturer` _returnvalue))
    (:`then_1`
      (bind _asurr_game_state_bp (cast `/Game/BluePrints/URR_GameState_BP` (`GameplayStatics.GetGameState`)))
      (set `self.GameState` _asurr_game_state_bp))))

(event `MoveRight`
  ;[1 1 1] MoveRight Axis (Update)
  (if (`self.GameStarted`)
    (`self.K2_SetActorLocation` (+ (`self.K2_GetActorLocation`) (* (`self.GetActorForwardVector`) (* (`self.Speed`) 1.0 (`GameplayStatics.GetWorldDeltaSeconds`)))) true)))

(event `MoveLeft`
  ;[1 1 1] MoveLeft
  (if (`self.GameStarted`)
    (`self.K2_SetActorLocation` (+ (`self.K2_GetActorLocation`) (* (`self.GetActorForwardVector`) (* (`self.Speed`) -1.0 (`GameplayStatics.GetWorldDeltaSeconds`)))) true)))

(event `self.ReceiveTick`
  (params (DeltaSeconds :type "Float (single-precision)"))
  ;[1 1 1] Choose Action
  (switch `int` (`self.action`)
    (:`1`
      (`self.MoveLeft`))
    (:`2`
      (`self.MoveRight`))))

(fn `UserConstructionScript`)