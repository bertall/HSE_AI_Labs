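; Ball Blueprint for a ball that moves by projectile movement and corrects its velocity when it hits something.
; On Hit, if the magnitude of either X or Z velocity falls below its minimum, both are replaced with random speeds that keep their current signs.
; The replacement zeroes Y, keeping motion in the XZ plane, and uses a larger range for Z than for X.
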(event `self.ReceiveHit`
  (params (MyComp :type "PrimitiveComponent Object Reference") (Other :type "Actor Object Reference") (OtherComp :type "PrimitiveComponent Object Reference") (bSelfMoved :type Boolean) (HitLocation :type "Vector Structure") (HitNormal :type "Vector Structure") (NormalImpulse :type "Vector Structure") (Hit :type "HitResult Structure (by ref)"))
  ;[1 1 1] Hit Event
  (bind _output_get (set `self.Temp_Velocity` (`self.GetVelocity`)))
  (if (or (< (`KismetMathLibrary.Abs` (.x _output_get)) 150.0) (< (`KismetMathLibrary.Abs` (.z _output_get)) 200.0))
    (set `MovementComponent.Velocity` (`KismetMathLibrary.MakeVector` (* (`KismetMathLibrary.SignOfFloat` (.x (`self.Temp_Velocity`))) (`KismetMathLibrary.RandomFloatInRange` 150.0 200.0)) 0.0 (* (`KismetMathLibrary.SignOfFloat` (.z (`self.Temp_Velocity`))) (`KismetMathLibrary.RandomFloatInRange` 600.0 800.0))) (`self.ProjectileMovement1`))))

(fn `UserConstructionScript`)