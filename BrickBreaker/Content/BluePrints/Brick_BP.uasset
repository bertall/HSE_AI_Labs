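; Brick_BP is a breakable Paper2D brick that destroys itself when hit by a Ball_BP.
; A hit decrements the game state's BricksCount and adds score, while violet bricks, given a purple sprite by the construction script, award more points plus a life.
; A separate SpawnBonus event, not called within this Blueprint, optionally randomizes the bonus type and spawns a randomly rotated Bonus_BP when that type is non-zero.
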(event `SpawnBonus`
  ;[1 1 1] Spawn Bonus Custom event
  (if (`self.RandomBonus`)
    (set `self.BonusType` (cast `/Game/BluePrints/Enums/BonusType` (`KismetMathLibrary.Conv_IntToByte` (`KismetMathLibrary.RandomIntegerInRange` 0 2)))))
  (if (!= (`self.BonusType`) 0)
    (bind _returnvalue (`|SpawnActorFromClass` "/Game/BluePrints/Bonus_Bp.Bonus_BP_C" (`KismetMathLibrary.MakeTransform` (`self.K2_GetActorLocation`) (`KismetMathLibrary.MakeRotator` 0.0 (`KismetMathLibrary.RandomFloatInRange` -180.0 180.0))) "AlwaysSpawn" "OverrideRootScale"))
    (`/Game/BluePrints/Bonus_Bp.SetBonus` _returnvalue (`self.BonusType`))))

(event `self.ReceiveHit`
  (params (MyComp :type "PrimitiveComponent Object Reference") (Other :type "Actor Object Reference") (OtherComp :type "PrimitiveComponent Object Reference") (bSelfMoved :type Boolean) (HitLocation :type "Vector Structure") (HitNormal :type "Vector Structure") (NormalImpulse :type "Vector Structure") (Hit :type "HitResult Structure (by ref)"))
  (bind _returnvalue (`GameplayStatics.GetGameState`))
  ;[1 1 1] hit Event
  (cast `/Game/BluePrints/Ball_BP` Other)
  (bind _asurr_game_state_bp (cast `/Game/BluePrints/URR_GameState_BP` (`GameplayStatics.GetGameState`)))
  (set `/Game/BluePrints/URR_GameState_BP.BricksCount` (- (`/Game/BluePrints/URR_GameState_BP.BricksCount` _asurr_game_state_bp) 1) _asurr_game_state_bp)
  (if (`self.isViolet`)
    (message `/Game/BluePrints/InterfacesBP/Score_Lives_BP_Interface.AddLives` _returnvalue 1)
    (message `/Game/BluePrints/InterfacesBP/Score_Lives_BP_Interface.UpdateScore` _returnvalue 100)
    (else
      (message `/Game/BluePrints/InterfacesBP/Score_Lives_BP_Interface.UpdateScore` _returnvalue 10)))
  (`self.K2_DestroyActor`))

(fn `UserConstructionScript`
  (if (`self.isViolet`)
    (`PaperSpriteComponent.SetSprite` (`self.PaperSprite1`) "/Game/Assets/NewFolder/element_purple_rectangle_Sprite.element_purple_rectangle_Sprite")))